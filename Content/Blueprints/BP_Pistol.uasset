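; BP_Pistol is a pistol Blueprint that fires projectiles and reloads, starting with a full magazine set in the construction script.
; Shoot spawns a BP_Ammo actor at the Arrow component's transform and decrements Ammo, printing the count or a Spanish out-of-ammo message when empty.
; Reload refills Ammo to MAXAMMO immediately, then holds an IsLoading flag through a short Delay to block shooting and repeat reloads.
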(event Custom|Shoot
  (if (not (Variables|Default|GetIsLoading))
    (if (> (Variables|Default|GetAmmo) 0)
      (Game|SpawnActorfromClass "/Game/Blueprints/BP_Ammo.BP_Ammo_C" (Transformation|GetWorldTransform (Variables|Default|GetArrow)) "Undefined" "MultiplyWithRoot" 0 0)
      (bind _result (Math|Integer|DecrementInt (Variables|Default|GetAmmo))
        (:%20%20
          (bind _output_get (Variables|Default|SetAmmo _result))
          (Development|PrintString (Utilities|String|ToString(Integer) _output_get))))
      (else
        (Development|PrintString "Sin munición")))))

(event Custom|Reload
  (if (not (Variables|Default|GetIsLoading))
    (Development|PrintString "Recargando")
    (Variables|Default|SetIsLoading true)
    (Variables|Default|SetAmmo (Variables|Default|GetMAX_AMMO))
    (Utilities|FlowControl|Delay 2.0)
    (Variables|Default|SetIsLoading false)))

(fn ConstructionScript
  (Variables|Default|SetAmmo (Variables|Default|GetMAX_AMMO)))