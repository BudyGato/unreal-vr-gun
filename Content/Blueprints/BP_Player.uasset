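; Player Blueprint that lets the player pick up a pistol, then shoot and reload it through Enhanced Input.
; BeginPlay adds the pistol mapping context.
; The first right mesh overlap with a pistol destroys it, spawns a replacement attached to that mesh, hides the mesh and shows the ammo widget.
; The pickup sets HasGun, which gates forwarding shoot and reload input to the gun.
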(event OnComponentBeginOverlap(StaticMesh_R)
  (params (OverlappedComponent :type Primitive%20Component%20Object%20Reference) (OtherActor :type Actor%20Object%20Reference) (OtherComp :type Primitive%20Component%20Object%20Reference) (OtherBodyIndex :type Integer) (bFromSweep :type Boolean) (SweepResult :type Hit%20Result%20Structure%20%28by%20ref%29))
  (bind _asbp_pistol (Utilities|Casting|CastToBP_Pistol OtherActor))
  (Utilities|FlowControl|DoOnce false
    (:Completed
      (Actor|DestroyActor _asbp_pistol)
      (Development|SetHiddeninGame (Variables|Default|GetStaticMesh_R) false false)
      (bind _returnvalue (Game|SpawnActorfromClass "/Game/Blueprints/BP_Pistol.BP_Pistol_C" (Transformation|GetWorldTransform (Variables|Default|GetStaticMesh_R)) "Undefined" "MultiplyWithRoot" 0 0))
      (bind _output_get (Variables|Default|SetGun _returnvalue))
      (Transformation|AttachComponentToComponent _output_get (Variables|Default|GetStaticMesh_R) "None" "SnapToTarget" "SnapToTarget" "SnapToTarget" true)
      (Rendering|SetVisibility (Variables|Default|GetStaticMesh_R) false false)
      (Rendering|SetVisibility (Variables|Default|GetAmmoWidget) true false)
      (Variables|Default|SetbHasGun true))))

(event Input|EnhancedActionEvents|EnhancedInputActionIA_Shoot
  (params (ActionValue :type Boolean) (ElapsedSeconds :type Float%20%28double-precision%29) (TriggeredSeconds :type Float%20%28double-precision%29) (InputAction :type Input%20Action%20Object%20Reference :default "/Game/Input/IA_Shoot.IA_Shoot"))
  (CallFunction|OnShoot))

(event Input|EnhancedActionEvents|EnhancedInputActionIA_Reload
  (params (ActionValue :type Boolean) (ElapsedSeconds :type Float%20%28double-precision%29) (TriggeredSeconds :type Float%20%28double-precision%29) (InputAction :type Input%20Action%20Object%20Reference :default "/Game/Input/IA_Reload.IA_Reload"))
  (:Started
    (if (Variables|Default|GetbHasGun)
      (Default|Reload (Variables|Default|GetGun)))))

(event EventBeginPlay
  (Input|AddMappingContext (PlayerController|LocalPlayerSubsystems|GetEnhancedInputLocalPlayerSubsystem (Game|GetPlayerController 0)) "/Game/Input/MC_Pistol.MC_Pistol" 0 "(bIgnoreAllPressedKeysUntilRelease=True,bForceImmediately=False,bNotifyUserSettings=False)"))

(event EventOnShoot
  (if (Variables|Default|GetbHasGun)
    (Default|Shoot (Variables|Default|GetGun))))

(fn ConstructionScript)