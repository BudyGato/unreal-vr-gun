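; BP_Enemy is an enemy actor that launches itself upward with a randomized look when play begins.
; BeginPlay assigns its StaticMesh from RandomMesh, a three-way random select in which only the Cone option names a mesh.
; It then applies a random rotation and uniform scale at the current relative location, and adds a random upward impulse as a velocity change, independent of mass.
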(event EventBeginPlay
  (Components|StaticMesh|SetStaticMesh (Variables|Default|GetStaticMesh) (CallFunction|RandomMesh))
  (Transformation|SetRelativeTransform (Variables|Default|GetStaticMesh) (Math|Transform|MakeTransform (Variables|/Script/Engine.SceneComponent|GetRelativeLocation (Variables|Default|GetStaticMesh)) (Math|Random|RandomRotator true) (Math|Conversions|ToVector(Float) (Math|Random|RandomFloatinRange 0.4 1.0))) false false)
  (Physics|AddImpulse (Variables|Default|GetStaticMesh) (Math|Vector|MakeVector 0.0 0.0 (Math|Random|RandomFloatinRange 7e+02 1.2e+03)) "None" true))

(fn ConstructionScript)

(fn RandomMesh
  (return (Utilities|Select :Index (Math|Random|RandomIntegerinRange 0 2) :Option%200 "/Engine/BasicShapes/Cone.Cone" :Option%201 0 :Option%202 0)))